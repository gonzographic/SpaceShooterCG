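; BP_PlayerShieldComponent is a component that switches the player's shield on and off in the space shooter.
; ActivateShield sets the active flag only if the component is neither disabled nor already active, while DeactivateShield clears it unconditionally.
; Both play a 2D sound and send ShieldVisibilityChangedMessage to the owner to show or hide the shield.
; Disable sets Disabled to false, so despite its name it leaves activation allowed.
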(fn `ActivateShield`
  ;[1 1 1] Check disabled
  (if (not (`self.Disabled`))
    ;[1 1 1] Check variable and set active when inactive
    (if (not (`self.IsShieldActive`))
      (set `self.IsShieldActive` true)
      ;[1 1 1] Play shield up sound
      (`GameplayStatics.PlaySound2D` (`self.ShieldUpSound`))
      ;[1 1 1] Show shield
      (message `/Game/SpaceShooter2DKit/Blueprints/Player/I_ShieldActor.ShieldVisibilityChanged` (`self.GetOwner`) true))))

(fn `DeactivateShield`
  ;[1 1 1] Reset variable
  (set `self.IsShieldActive` false)
  ;[1 1 1] Play shield down sound
  (`GameplayStatics.PlaySound2D` (`self.ShieldDownSound`))
  ;[1 1 1] Hide shield
  (message `/Game/SpaceShooter2DKit/Blueprints/Player/I_ShieldActor.ShieldVisibilityChanged` (`self.GetOwner`) false))

(fn `Disable`
  (set `self.Disabled` false))