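; Player ship for a 2D space shooter, built on a base character, that applies the selected ship's flipbooks, scale and collision from a data table.
; Input and Tick drive separate movement, shooting and nuke components.
; An active shield component absorbs one hit, then deactivates.
; On death it disables those components, plays the death flipbook under altered global time dilation, hides the actor and notifies the GameMode of game over.
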(event `self.ReceiveBeginPlay`
  (`self.SetPlayerShipVisuals`))

(event `/Game/SpaceShooter2DKit/Blueprints/Player/I_ShieldActor.ShieldVisibilityChanged`
  (params (IsVisible :type Boolean))
  (`SceneComponent.SetVisibility` (`self.ShieldFlipbook`) IsVisible false))

(event `/Game/SpaceShooter2DKit/Blueprints/Components/I_HealthActor.OnHit`
  (`GameplayStatics.PlaySound2D` (`self.HitSound`) 1.0 1.0 0.0 null null))

(event `InputAction|Fire`
  (params (Key :type "Key Structure"))
  ;[1 1 1] disparo
  (:`Pressed`
    (`/Game/SpaceShooter2DKit/Blueprints/Player/BP_PlayerShootingComponent.OnFirePressed` (`self.BP_PlayerShootingComponent`)))
  (:`Released`
    (`/Game/SpaceShooter2DKit/Blueprints/Player/BP_PlayerShootingComponent.OnFireReleased` (`self.BP_PlayerShootingComponent`))))

(event `self.ReceiveTick`
  (params (DeltaSeconds :type "Float (single-precision)"))
  (`/Game/SpaceShooter2DKit/Blueprints/Player/BP_PlayerMovementComponent.ApplyMovementInput` (`self.BP_PlayerMovementComponent`) DeltaSeconds (`self.GetInputAxisValue`) (`self.GetInputAxisValue`)))

(event `InputAction|Nuke`
  (params (Key :type "Key Structure"))
  ;[1 1 1] nuke
  (:`Pressed`
    (`/Game/SpaceShooter2DKit/Blueprints/Player/BP_PlayerNukeComponent.ActivateNuke` (`self.BP_PlayerNukeComponent`))))

(event `/Game/SpaceShooter2DKit/Blueprints/Components/I_HealthActor.OnDeath`
  ;[1 1 1] muerte
  (`|ExecutionSequence`
    (:`then_0`
      (`self.DisableComponents`))
    (:`then_1`
      (`GameplayStatics.SetGlobalTimeDilation` (`self.DeathTimeDilationFactor`))
      (`self.StartDeathAnimation`)
      (`KismetSystemLibrary.Delay` (`PaperFlipbookComponent.GetFlipbookLength` (`self.Sprite`)))
      (`self.SetActorHiddenInGame` true)
      (`GameplayStatics.SetGlobalTimeDilation` 1.0))
    (:`then_2`
      (bind _asbp_space_shooter_2dgame_mode (cast `/Game/SpaceShooter2DKit/Blueprints/Game/BP_SpaceShooter2DGameMode` (`GameplayStatics.GetGameMode`)))
      (`/Game/SpaceShooter2DKit/Blueprints/Game/BP_SpaceShooter2DGameMode.GameOver` _asbp_space_shooter_2dgame_mode))))

(fn `DisableComponents`
  (`/Game/SpaceShooter2DKit/Blueprints/Player/BP_PlayerMovementComponent.Disable` (`self.BP_PlayerMovementComponent`))
  (`/Game/SpaceShooter2DKit/Blueprints/Player/BP_PlayerShootingComponent.Disable` (`self.BP_PlayerShootingComponent`))
  (`/Game/SpaceShooter2DKit/Blueprints/Player/BP_PlayerNukeComponent.Disable` (`self.BP_PlayerNukeComponent`))
  (`/Game/SpaceShooter2DKit/Blueprints/Player/BP_PlayerShieldComponent.Disable` (`self.BP_PlayerShieldComponent`)))

(fn `SetPlayerShipVisuals`
  (locals (ShipData :type "/Game/SpaceShooter2DKit/Blueprints/Player/STR_PlayerShip Structure"))
  ;[1 1 1] Get selected player shp from Game Instance
  (bind _asbp_space_shooter_2dgame_instance (cast `/Game/SpaceShooter2DKit/Blueprints/Game/BP_SpaceShooter2DGameInstance` (`GameplayStatics.GetGameInstance`)))
  (bind _returnvalue (`|GetDataTableRow` "/Game/SpaceShooter2DKit/Blueprints/Player/DT_PlayerShips.DT_PlayerShips" (`/Game/SpaceShooter2DKit/Blueprints/Game/BP_SpaceShooter2DGameInstance.SelectedShip` _asbp_space_shooter_2dgame_instance))
    (:`then`
      (set `local.ShipData` _returnvalue)
      (`|ExecutionSequence`
        (:`then_0`
          ;[1 1 1] Update Ship Flipbook
          (`PaperFlipbookComponent.SetFlipbook` (`self.Sprite`) (`.Flipbook_26_C7EB8D8C4ACD0F3D614C9095A0FE6AC4` (break `/Game/SpaceShooter2DKit/Blueprints/Player/STR_PlayerShip` (`local.ShipData`)))))
        (:`then_1`
          ;[1 1 1] Update Engine Flipbook
          (`PaperFlipbookComponent.SetFlipbook` (`self.EngineFlipbook`) (`.EngineFlipbook_40_9175CC0144B1FD814921C3B05B924D53` (break `/Game/SpaceShooter2DKit/Blueprints/Player/STR_PlayerShip` (`local.ShipData`)))))
        (:`then_2`
          ;[1 1 1] Update Shield Flipbook
          (`PaperFlipbookComponent.SetFlipbook` (`self.ShieldFlipbook`) (`.ShieldFlipbook_41_45A6137B454A41F44ECA39BE3A0A9B3F` (break `/Game/SpaceShooter2DKit/Blueprints/Player/STR_PlayerShip` (`local.ShipData`)))))
        (:`then_3`
          ;[1 1 1] Update Death Flipbook
          (set `self.DeathAnimation` (`.DeathFlipbook_39_8F9B51A24608F9D27F2263980B39EEE4` (break `/Game/SpaceShooter2DKit/Blueprints/Player/STR_PlayerShip` (`local.ShipData`)))))
        (:`then_4`
          ;[1 1 1] Update Flipbook scale
          (`SceneComponent.SetRelativeScale3D` (`self.Sprite`) (`.Scale_23_768DFF224EAD7DDB4F0BE082CB0A54D5` (break `/Game/SpaceShooter2DKit/Blueprints/Player/STR_PlayerShip` (`local.ShipData`)))))
        (:`then_5`
          ;[1 1 1] Update Box Collision Extends
          (`BoxComponent.SetBoxExtent` (`self.Box`) (`.BoxCollisionExtend_32_5CB36B2E41E520DA9A6802B1FCD9B6D0` (break `/Game/SpaceShooter2DKit/Blueprints/Player/STR_PlayerShip` (`local.ShipData`))) true))))
    (:`RowNotFound`
      ;[1 1 1] Print error when ship is not found
      (`KismetSystemLibrary.PrintString` "Selected Ship not found in DataTable"))))

(fn `ShouldIgnoreDamage`
  (returns (IgnoreDamage :type Boolean))
  (if (`/Game/SpaceShooter2DKit/Blueprints/Player/BP_PlayerShieldComponent.IsShieldActive` (`self.BP_PlayerShieldComponent`))
    ;[1 1 1] If active, ignore the hit and deactivate shield
    (`/Game/SpaceShooter2DKit/Blueprints/Player/BP_PlayerShieldComponent.DeactivateShield` (`self.BP_PlayerShieldComponent`))
    (return true)
    (else
      (return false))))

(fn `StartDeathAnimation`
  ;[1 1 1] Change the flipbook
  (`PaperFlipbookComponent.SetFlipbook` (`self.Sprite`) (`self.DeathAnimation`))
  ;[1 1 1] Hide Engine Flipbook
  (`SceneComponent.SetVisibility` (`self.EngineFlipbook`) false false))

(fn `UserConstructionScript`
  ;[1 1 1] Call constructor script of BaseCharacter
  (`parent.UserConstructionScript`))