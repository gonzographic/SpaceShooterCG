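; Player component that provides a limited-ammo nuke, a screen-clearing attack against enemies in the 2D space shooter.
; ActivateNuke checks that the component is enabled and has ammo, spends one charge, then applies nuke damage from the owner to every BP_BaseEnemy actor in the world.
; Ammo changes are clamped between zero and the maximum, and Disable blocks further activation.
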(fn `ActivateNuke`
  ;[1 1 1] Check if nuke can be activated
  (if (`self.CanActivateNuke`)
    ;[1 1 1] Reduce ammo with 1
    (`self.ChangeNukeAmmo` -1)
    ;[1 1 1] Loop through all enemies
    (bind _outactors (`GameplayStatics.GetAllActorsOfClass` "/Game/SpaceShooter2DKit/Blueprints/Enemies/BP_BaseEnemy.BP_BaseEnemy_C"))
    (for _array_element _outactors
      ;[1 1 1] Apply nuke damage to each enemy
      (`GameplayStatics.ApplyDamage` _array_element (`self.NukeDamage`) null (`self.GetOwner`)))))

(fn `CanActivateNuke`
  (returns (CanActivate :type Boolean))
  (return (and (not (`self.Disabled`)) (> (`self.CurrentNukeAmmo`) 0))))

(fn `ChangeNukeAmmo`
  (params (Delta :type Integer))
  (set `self.CurrentNukeAmmo` (`KismetMathLibrary.Clamp` (+ (`self.CurrentNukeAmmo`) (`local.Delta`)) 0 (`self.MaxNukeAmmo`))))

(fn `Disable`
  (set `self.Disabled` true))