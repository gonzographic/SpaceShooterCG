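; Health component that gives its owning actor health, armor, damage handling, death state and optional regeneration.
; It binds to the owner's damage event and skips hits in god mode, when dead, or when the owner opts out.
; Armor absorbs damage first; any overflow reduces health and sends hit or death messages to the owner.
; Health damage halts regeneration, and surviving actors restart it through a delay timer feeding a looping heal timer.
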(event `self.ReceiveBeginPlay`
  (`self.Initialize`)
  (add `Actor.OnTakeAnyDamage` (`self.GetOwner`) (delegate `HandleDamage`)))

(event `HandleDamage`
  (params (DamagedActor :type "Actor Object Reference") (Damage :type "Float (double-precision)") (DamageType :type "DamageType Object Reference") (InstigatedBy :type "Controller Object Reference") (DamageCauser :type "Actor Object Reference"))
  (if (`self.CanBeDamaged`)
    (`self.OnDamage` Damage)))

(fn `CanBeDamaged`
  (returns (CanBeDamaged :type Boolean))
  (if (`self.GodMode`)
    (return false)
    (elif (`self.IsDead`)
      (return false)
      (else
        (bind _ignoredamage (message `/Game/SpaceShooter2DKit/Blueprints/Components/I_HealthActor.ShouldIgnoreDamage` (`self.GetOwner`)))
        (return (not _ignoredamage))))))

(fn `ChangeArmor`
  (params (OriginalDelta :type "Float (double-precision)"))
  (returns (RemainingDelta :type "Float (double-precision)"))
  (locals (Diff :type "Float (double-precision)" :default 0.0))
  ;[1 1 1] Check reduce armor or add armor
  (if (< OriginalDelta 0.0)
    ;[1 1 1] Determine the difference between Damage and current Armor
    (bind _output_get (set `local.Diff` (+ (`self.CurrentArmor`) OriginalDelta)))
    (if (> _output_get 0.0)
      ;[1 1 1] If we had more armor than damage, reduce the armor and return 0
      (set `self.CurrentArmor` (`local.Diff`))
      (return 0.0)
      (else
        ;[1 1 1] Else armor is 0 and return the (absolute) difference
        (set `self.CurrentArmor` 0.0)
        (return (`KismetMathLibrary.Abs` (`local.Diff`)))))
    (else
      ;[1 1 1] Add the delta to CurrentArmor (clamped to MaxArmor) and return 0
      (set `self.CurrentArmor` (`KismetMathLibrary.FClamp` (+ (`self.CurrentArmor`) OriginalDelta) 0.0 (`self.MaxArmor`)))
      (return 0.0))))

(fn `ChangeHealth`
  (params (Delta :type "Float (double-precision)"))
  ;[1 1 1] If not already dead
  (if (not (`self.IsDead`))
    ;[1 1 1] Change health by delta (and clamp between 0 and max health)
    (set `self.CurrentHealth` (`KismetMathLibrary.FClamp` (+ (`self.CurrentHealth`) Delta) 0.0 (`self.MaxHealth`)))
    ;[1 1 1] Update dead after changing health
    (`self.UpdateDead`)))

(fn `ChangeMaxArmor`
  (params (NewMaxArmor :type "Float (double-precision)") (FullArmor :type Boolean))
  ;[1 1 1] Check not already dead
  (if (not (`self.IsDead`))
    ;[1 1 1] Update max health
    (set `self.MaxArmor` NewMaxArmor)
    ;[1 1 1] If Full Armor, update armor to max armor
    (if FullArmor
      (`self.ChangeArmor` (`self.MaxArmor`)))))

(fn `ChangeMaxHealth`
  (params (NewMaxHealth :type "Float (double-precision)") (FullHealth :type Boolean))
  ;[1 1 1] Check not already dead
  (if (not (`self.IsDead`))
    ;[1 1 1] Update max health
    (set `self.MaxHealth` NewMaxHealth)
    ;[1 1 1] If Full Health, heal actor to max health
    (if FullHealth
      (`self.ChangeHealth` (`self.MaxHealth`)))))

(fn `Initialize`
  ;[1 1 1] Set health to maximum
  (set `self.CurrentHealth` (`self.MaxHealth`))
  (if (`self.StartFullArmor`)
    ;[1 1 1] Set armor to maximum, if enabled
    (set `self.CurrentArmor` (`self.MaxArmor`))))

(fn `InitializeEnemyHealth`
  (params (MaxHealth :type "Float (double-precision)"))
  (`self.ChangeMaxHealth` MaxHealth true))

(fn `IsFullArmor`
  (returns (IsFullArmor :type Boolean))
  ;[1 1 1] Return whether the actor is full armor (health >= maximum health)
  (return (>= (`self.CurrentArmor`) (`self.MaxArmor`))))

(fn `IsFullHealth`
  (returns (IsFullHealth :type Boolean))
  ;[1 1 1] Return whether the actor is full health (health >= maximum health)
  (return (>= (`self.CurrentHealth`) (`self.MaxHealth`))))

(fn `OnDamage`
  (params (DamageAmount :type "Float (double-precision)"))
  (returns (Died :type Boolean))
  (locals (LocalDied :type Boolean :default false))
  (bind _returnvalue (`self.GetOwner`))
  (bind _remainingdelta (`self.ChangeArmor` (* DamageAmount -1.0)))
  (if (> _remainingdelta 0.0)
    (`|ExecutionSequence`
      (:`then_0`
        ;[1 1 1] Stop health regeneration
        (`self.StopRegeneration`))
      (:`then_1`
        ;[1 1 1] Subtract damage
        (`self.ChangeHealth` (* _remainingdelta -1.0)))
      (:`then_2`
        ;[1 1 1] Check dead
        (bind _isdead (`self.UpdateDead`))
        (bind _output_get (set `local.LocalDied` _isdead))
        (if _output_get
          (message `/Game/SpaceShooter2DKit/Blueprints/Components/I_HealthActor.OnDeath` _returnvalue)
          (else
            (message `/Game/SpaceShooter2DKit/Blueprints/Components/I_HealthActor.OnHit` _returnvalue)))
        ;[1 1 1] If true, return value. Else start health regen and return value
        (if (`local.LocalDied`)
          (return (`local.LocalDied`))
          (else
            ;[1 1 1] Can this actor regen health?
            (if (`self.CanRegen`)
              ;[1 1 1] Start health regen after regen delay
              (`KismetSystemLibrary.K2_SetTimer` null "StartRegeneration" (`self.RegenDelay`))
              (return (`local.LocalDied`)))))))))

(fn `RegenHealth`
  ;[1 1 1] Add regen amount to current health
  (`self.ChangeHealth` (`self.RegenAmount`)))

(fn `StartRegeneration`
  (if (`self.CanRegen`)
    (`KismetSystemLibrary.K2_SetTimer` null "RegenHealth" (`self.RegenRate`) true)))

(fn `StopRegeneration`
  ;[1 1 1] Stop the start timer
  (`KismetSystemLibrary.K2_ClearTimer` null "StartRegeneration")
  ;[1 1 1] Stop the current regen
  (`KismetSystemLibrary.K2_ClearTimer` null "RegenHealth"))

(fn `UpdateDead`
  (returns (IsDead :type Boolean))
  ;[1 1 1] Check whether character is dead (health <= 0)
  (bind _output_get (set `self.IsDead` (<= (`self.CurrentHealth`) 0.0)))
  (return _output_get))