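; Enemy component that makes its owner periodically dodge up or down in the 2D shooter.
; Initialize takes the evade properties and, if evasion is allowed, starts a looping timer after an optional delay, its interval randomized once.
; Each Evade adds a random vertical direction to the owner's BP_EnemyMovementComponent for a set duration, guarded against overlap.
; Disable clears both timers.
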(event `Evade`
  ;[1 1 1] Avoid double evade
  (if (not (`self.IsEvading`))
    (set `self.IsEvading` true)
    ;[1 1 1] Start evade movement
    (`self.StartEvade`)
    ;[1 1 1] Wait evade duration
    (`KismetSystemLibrary.Delay` (`.EvadeDuration_20_C0738575C04C560FD681548EF9417462` (break `/Game/SpaceShooter2DKit/Blueprints/Enemies/STR_EnemyEvadeProperties` (`self.EvadeProperties`))))
    ;[1 1 1] Stop evade movement
    (`self.StopEvade`)
    ;[1 1 1] Reset variable
    (set `self.IsEvading` false)))

(fn `Disable`
  ;[1 1 1] Stop both timers to stop evading
  (`KismetSystemLibrary.K2_ClearTimer` null "StartEvading")
  (`KismetSystemLibrary.K2_ClearTimer` null "Evade"))

(fn `Initialize`
  (params (EvadeProperties :type "/Game/SpaceShooter2DKit/Blueprints/Enemies/STR_EnemyEvadeProperties Structure"))
  (set `self.EvadeProperties` EvadeProperties)
  ;[1 1 1] Can the enemy evade?
  (if (`.CanEvade_16_AEF4DBAFDB40D4C0E8C770B50D4AAE79` (break `/Game/SpaceShooter2DKit/Blueprints/Enemies/STR_EnemyEvadeProperties` (`self.EvadeProperties`)))
    ;[1 1 1] No delay means start evading now
    (if (<= (`.InitialEvadeDelay_17_DCFF6F081947C0DB0F6C43BF1DBE2639` (break `/Game/SpaceShooter2DKit/Blueprints/Enemies/STR_EnemyEvadeProperties` (`self.EvadeProperties`))) 0.0)
      ;[1 1 1] Start evading now
      (`self.StartEvading`)
      (else
        ;[1 1 1] Set the timer to start evading
        (`KismetSystemLibrary.K2_SetTimer` null "StartEvading" (`.InitialEvadeDelay_17_DCFF6F081947C0DB0F6C43BF1DBE2639` (break `/Game/SpaceShooter2DKit/Blueprints/Enemies/STR_EnemyEvadeProperties` (`self.EvadeProperties`))))))))

(fn `StartEvade`
  (bind _returnvalue (`Actor.GetComponentByClass` (`self.GetOwner`) "/Game/SpaceShooter2DKit/Blueprints/Enemies/BP_EnemyMovementComponent.BP_EnemyMovementComponent_C"))
  (`/Engine/EditorBlueprintResources/StandardMacros.IsValid` _returnvalue
    (:`Is Valid`
      (`/Game/SpaceShooter2DKit/Blueprints/Enemies/BP_EnemyMovementComponent.SetDirectionAddition` _returnvalue (select `bool` (`KismetMathLibrary.RandomBool`) :`false` (0.0 0.0 -1.0) :`true` (0.0 0.0 1.0) :!type "Vector Structure")))))

(fn `StartEvading`
  (bind ((`MinEvadeDelay_22_5324E9844E47AC58CE24A69B565D7D78` _minevadedelay) (`MaxEvadeDelay_19_095C13D4AD474F92D07E0D9D20232C50` _maxevadedelay)) (break `/Game/SpaceShooter2DKit/Blueprints/Enemies/STR_EnemyEvadeProperties` (`self.EvadeProperties`)))
  ;[1 1 1] Setup timer with Min and Max delay time. Looping to keep evading
  (`KismetSystemLibrary.K2_SetTimer` null "Evade" (`KismetMathLibrary.RandomFloatInRange` _minevadedelay _maxevadedelay) true))

(fn `StopEvade`
  (bind _returnvalue (`Actor.GetComponentByClass` (`self.GetOwner`) "/Game/SpaceShooter2DKit/Blueprints/Enemies/BP_EnemyMovementComponent.BP_EnemyMovementComponent_C"))
  (`/Engine/EditorBlueprintResources/StandardMacros.IsValid` _returnvalue
    (:`Is Valid`
      (`/Game/SpaceShooter2DKit/Blueprints/Enemies/BP_EnemyMovementComponent.ClearDirectionAddition` _returnvalue))))