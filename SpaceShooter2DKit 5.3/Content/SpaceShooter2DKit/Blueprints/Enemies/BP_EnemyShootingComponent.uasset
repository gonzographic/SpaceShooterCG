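; Enemy shooting component for a 2D shooter that periodically fires projectiles from configured eject points on its owning actor.
; Initialize stores the shoot properties and starts a looping Fire timer, randomizing the reload interval once; Disable clears it.
; Fire spawns an enemy torpedo projectile per point, offset along its fire direction.
; Depending on shoot mode, shots aim at the player while the enemy's X is greater, otherwise follow the rotated forward vector.
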(fn `Disable`
  ;[1 1 1] Clear the Timer for Fire function
  (`KismetSystemLibrary.K2_ClearTimer` null "Fire"))

(fn `Fire`
  (for _array_element (`.ProjectileEjectPoints_24_71664EFB8B4A88C9A5F4E1B9CCF2DD01` (break `/Game/SpaceShooter2DKit/Blueprints/Enemies/STR_EnemyShootProperties` (`self.ShootProperties`)))
    (bind (_verticaloffset _spawnoffset _anglefromforward) (break `/Game/SpaceShooter2DKit/Blueprints/Player/STR_EjectInfo` _array_element))
    (bind _firedirection (`self.GetFireDirection` _anglefromforward))
    ;[1 1 1] Spawn projectiles
    (`|SpawnActorFromClass` "/Game/SpaceShooter2DKit/Blueprints/Projectiles/BP_Projectile.BP_Projectile_C" (`KismetMathLibrary.MakeTransform` (+ (`Actor.K2_GetActorLocation` (`self.GetOwner`)) (+ (* (`Actor.GetActorUpVector` (`self.GetOwner`)) _verticaloffset) (* _firedirection _spawnoffset))) (struct) (2.0 2.0 2.0)) "Undefined" "OverrideRootScale" null _firedirection (`.ProjectileDamage_38_291718044D1844794B2B1FB166DE8B98` (break `/Game/SpaceShooter2DKit/Blueprints/Enemies/STR_EnemyShootProperties` (`self.ShootProperties`))) "ECC_GameTraceChannel4" "/Game/SpaceShooter2DKit/Animations/Projectiles/FB_EnemyTorpedo.FB_EnemyTorpedo" null)))

(fn `GetFireDirection`
  (params (AngleFromForward :type "Float (double-precision)"))
  (returns (FireDirection :type "Vector Structure"))
  (return (select `bool` (and (`|EnumEquality` (`.ShootDirection_29_FE5CB7FC2040C16890087EA15E787D89` (break `/Game/SpaceShooter2DKit/Blueprints/Enemies/STR_EnemyShootProperties` (`self.ShootProperties`))) "NewEnumerator1") (`self.IsInFrontOfPlayer`)) :`false` (`KismetMathLibrary.RotateAngleAxis` (`Actor.GetActorForwardVector` (`self.GetOwner`)) AngleFromForward (`Actor.GetActorRightVector` (`self.GetOwner`))) :`true` (`self.GetPlayerDirection`))))

(fn `GetPlayerDirection`
  (returns (PlayerDirection :type "Vector Structure"))
  (return (`KismetMathLibrary.Normal` (- (`Actor.K2_GetActorLocation` (`GameplayStatics.GetPlayerPawn` 0)) (`Actor.K2_GetActorLocation` (`self.GetOwner`))))))

(fn `Initialize`
  (params (ShootProperties :type "/Game/SpaceShooter2DKit/Blueprints/Enemies/STR_EnemyShootProperties Structure"))
  (bind (_lowerbound _upperbound) (break `FloatRange` (`.ReloadTime_27_103085DF4F0590B977DE80A1F1615DE6` (break `/Game/SpaceShooter2DKit/Blueprints/Enemies/STR_EnemyShootProperties` (`self.ShootProperties`)))))
  (set `self.ShootProperties` ShootProperties)
  ;[1 1 1] Can the enemy shoot?
  (if (> (`KismetArrayLibrary.Array_Length` (`.ProjectileEjectPoints_24_71664EFB8B4A88C9A5F4E1B9CCF2DD01` (break `/Game/SpaceShooter2DKit/Blueprints/Enemies/STR_EnemyShootProperties` (`self.ShootProperties`)))) 0)
    ;[1 1 1] Setup timer with Min and Max reload time. Looping to keep shooting
    (`KismetSystemLibrary.K2_SetTimer` null "Fire" (`KismetMathLibrary.RandomFloatInRange` (`.Value` (break `FloatRangeBound` _lowerbound)) (`.Value` (break `FloatRangeBound` _upperbound))) true)))

(fn `IsInFrontOfPlayer`
  (returns (IsInFront :type Boolean))
  (return (> (.x (`Actor.K2_GetActorLocation` (`self.GetOwner`))) (.x (`Actor.K2_GetActorLocation` (`GameplayStatics.GetPlayerPawn` 0))))))