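; Enemy spawner Blueprint that spawns one enemy type while its count in the level stays below a maximum.
; Activate starts a looping timer at the spawnees-per-second rate, and Deactivate clears it.
; Each tick of the timer gathers all BP_BaseEnemy actors, filters them by the configured type, and spawns another with the configured type and scale if under the limit.
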(event `/Game/SpaceShooter2DKit/Blueprints/Spawners/I_Spawner.Activate`
  (`KismetSystemLibrary.K2_SetTimer` null "SpawnEnemy" (/ 1.0 (`self.SpawneesPerSecond`)) true))

(event `/Game/SpaceShooter2DKit/Blueprints/Spawners/I_Spawner.Deactivate`
  (`KismetSystemLibrary.K2_ClearTimer` null "SpawnEnemy"))

(event `SpawnEnemy`
  (bind (_spawneeclass_type _spawneeclass_scale) (break `/Game/SpaceShooter2DKit/Blueprints/Spawners/STR_EnemySpawnee` (`self.SpawneeClass`)))
  (bind _outactors (`GameplayStatics.GetAllActorsOfClass` "/Game/SpaceShooter2DKit/Blueprints/Enemies/BP_BaseEnemy.BP_BaseEnemy_C"))
  (bind _filteredenemies (`self.FilterOnType` _outactors (`.Type_6_155FAFCB0F403035815DB095C42204E4` (break `/Game/SpaceShooter2DKit/Blueprints/Spawners/STR_EnemySpawnee` (`self.SpawneeClass`)))))
  (if (< (`KismetArrayLibrary.Array_Length` _filteredenemies) (`self.MaxSpawneesInLevel`))
    (`self.SpawnEnemyType` _spawneeclass_type _spawneeclass_scale)))

(fn `UserConstructionScript`)