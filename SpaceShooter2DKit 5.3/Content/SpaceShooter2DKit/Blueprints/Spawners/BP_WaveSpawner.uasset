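; BP_WaveSpawner is a spawner in the 2D space shooter kit that releases enemies in repeating timed waves.
; Activate starts a looping timer whose SpawnEnemy event passes a random Spawnees entry's type and scale to SpawnEnemyType, up to SpawneesPerWave times.
; After each wave it clears the timer, waits WaveDelay and sends itself Activate again unless Deactivate has set the Deactivated flag.
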(event `/Game/SpaceShooter2DKit/Blueprints/Spawners/I_Spawner.Activate`
  (if (> (`KismetArrayLibrary.Array_Length` (`self.Spawnees`)) 0)
    (`KismetSystemLibrary.K2_SetTimer` null "SpawnEnemy" (`self.EnemyDelay`) true)
    ;[1 1 1] Reset Deactivated
    (set `self.Deactivated` false)
    (else
      (`KismetSystemLibrary.PrintString` "Add Spawnees to WaveSpawener"))))

(event `/Game/SpaceShooter2DKit/Blueprints/Spawners/I_Spawner.Deactivate`
  (`KismetSystemLibrary.K2_ClearTimer` null "SpawnEnemy")
  (set `self.Deactivated` true))

(event `SpawnEnemy`
  (if (< (`self.CurrentSpawneeIndex`) (`self.SpawneesPerWave`))
    (bind _actortospawn (`self.GetRandomSpawnee`))
    (`self.SpawnEnemyType` (break `/Game/SpaceShooter2DKit/Blueprints/Spawners/STR_EnemySpawnee` _actortospawn) (`.Scale_5_F49C72B72D4D85DDA355C5A9587ED53E` (break `/Game/SpaceShooter2DKit/Blueprints/Spawners/STR_EnemySpawnee` _actortospawn)))
    (`/Engine/EditorBlueprintResources/StandardMacros.IncrementInt` (`self.CurrentSpawneeIndex`))
    (else
      (`KismetSystemLibrary.K2_ClearTimer` null "SpawnEnemy")
      (set `self.CurrentSpawneeIndex` 0)
      (`KismetSystemLibrary.Delay` (`self.WaveDelay`))
      (if (not (`self.Deactivated`))
        (message `/Game/SpaceShooter2DKit/Blueprints/Spawners/I_Spawner.Activate` self)))))

(fn `GetRandomSpawnee`
  (returns (ActorToSpawn :type "/Game/SpaceShooter2DKit/Blueprints/Spawners/STR_EnemySpawnee Structure"))
  (return (`|GetArrayItem` (`self.Spawnees`) (`KismetMathLibrary.RandomIntegerInRange` 0 (- (`KismetArrayLibrary.Array_Length` (`self.Spawnees`)) 1)))))

(fn `UserConstructionScript`)