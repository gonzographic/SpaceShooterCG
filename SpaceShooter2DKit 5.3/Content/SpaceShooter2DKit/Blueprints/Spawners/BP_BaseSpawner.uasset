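; Base spawner for the 2D space shooter kit that, when enabled, sends an Activate message after an initial delay on BeginPlay.
; It provides helpers to spawn any actor class, or a BP_BaseEnemy of a given type with a default rotation, at random points within SpawnArea bounds.
; A further helper filters enemy lists by type.
; The file contains no activation logic or spawn loop of its own.
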(event `self.ReceiveBeginPlay`
  (if (`self.Enabled`)
    (`KismetSystemLibrary.Delay` (`self.InitialDelay`))
    (message `/Game/SpaceShooter2DKit/Blueprints/Spawners/I_Spawner.Activate` self)))

(fn `FilterOnType`
  (params (UnfilteredEnemies :type "Array of /Game/SpaceShooter2DKit/Blueprints/Enemies/BP_BaseEnemy Object Reference") (Type :type "/Game/SpaceShooter2DKit/Blueprints/Enemies/ENUM_EnemyType Enum" :default "NewEnumerator0"))
  (returns (FilteredEnemies :type "Array of /Game/SpaceShooter2DKit/Blueprints/Enemies/BP_BaseEnemy Object Reference"))
  (locals (Result :type "Array of /Game/SpaceShooter2DKit/Blueprints/Enemies/BP_BaseEnemy Object Reference"))
  (for _array_element UnfilteredEnemies
    (if (`/Game/SpaceShooter2DKit/Blueprints/Enemies/BP_BaseEnemy.HasType` _array_element Type)
      (`KismetArrayLibrary.Array_Add` (`local.Result`) _array_element)))
  (return (`local.Result`)))

(fn `GetRandomSpawnPoint`
  (returns (RandomSpawnpoint :type "Vector Structure"))
  (bind _spawnarea (`self.SpawnArea`))
  (return (`KismetMathLibrary.MakeVector` (`KismetMathLibrary.RandomFloatInRange` (.x (break `/Game/SpaceShooter2DKit/Blueprints/Spawners/STR_SpawnArea` _spawnarea)) (.x (`.MaximumCoordinates_13_72D42F28E14888D7781FD4858CDB8A28` (break `/Game/SpaceShooter2DKit/Blueprints/Spawners/STR_SpawnArea` _spawnarea)))) (`KismetMathLibrary.RandomFloatInRange` (.y (break `/Game/SpaceShooter2DKit/Blueprints/Spawners/STR_SpawnArea` _spawnarea)) (.y (`.MaximumCoordinates_13_72D42F28E14888D7781FD4858CDB8A28` (break `/Game/SpaceShooter2DKit/Blueprints/Spawners/STR_SpawnArea` _spawnarea)))) (`KismetMathLibrary.RandomFloatInRange` (.z (break `/Game/SpaceShooter2DKit/Blueprints/Spawners/STR_SpawnArea` _spawnarea)) (.z (`.MaximumCoordinates_13_72D42F28E14888D7781FD4858CDB8A28` (break `/Game/SpaceShooter2DKit/Blueprints/Spawners/STR_SpawnArea` _spawnarea)))))))

(fn `SpawnActor`
  (params (Class :type "Actor Class Reference") (Rotation :type "Rotator Structure") (Scale :type "Vector Structure"))
  (returns (SpawnedActor :type "Actor Object Reference"))
  (bind _returnvalue (`|SpawnActorFromClass` Class (`KismetMathLibrary.MakeTransform` (`self.GetRandomSpawnPoint`) (`local.Rotation`) (`local.Scale`)) "Undefined" "SelectDefaultAtRuntime" null null))
  (return _returnvalue))

(fn `SpawnEnemyType`
  (params (Type :type "/Game/SpaceShooter2DKit/Blueprints/Enemies/ENUM_EnemyType Enum" :default "NewEnumerator0") (Scale :type "Vector Structure"))
  (returns (SpawnedEnemy :type "/Game/SpaceShooter2DKit/Blueprints/Enemies/BP_BaseEnemy Object Reference"))
  (locals (DefaultEnemyRotation :type "Rotator Structure" :default (struct :`Yaw` -180.0)))
  (bind _returnvalue (`|SpawnActorFromClass` "/Game/SpaceShooter2DKit/Blueprints/Enemies/BP_BaseEnemy.BP_BaseEnemy_C" (`KismetMathLibrary.MakeTransform` (`self.GetRandomSpawnPoint`) (`local.DefaultEnemyRotation`) (`local.Scale`)) "AlwaysSpawn" "OverrideRootScale" null (`local.Type`) null))
  (return _returnvalue))

(fn `UserConstructionScript`)