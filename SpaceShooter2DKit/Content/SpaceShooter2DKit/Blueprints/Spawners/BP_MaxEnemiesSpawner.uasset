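; Spawner blueprint for a 2D space shooter that spawns enemies of a configured type while capping how many exist in the level.
; Activate starts a looping timer that calls SpawnEnemy at the spawnees-per-second rate, and Deactivate clears it.
; Each tick gathers all BP_BaseEnemy actors, filters them by the spawnee type, and spawns one at the configured scale only if that count is below the level maximum.
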(event `/Game/SpaceShooter2DKit/Blueprints/Spawners/I_Spawner.Activate`
  ;[1 1 1] Call SpawnEnemy to achive spawnees per second rate
  (`KismetSystemLibrary.K2_SetTimer` null "SpawnEnemy" (/ 1.0 (`self.SpawneesPerSecond`)) true))

(event `/Game/SpaceShooter2DKit/Blueprints/Spawners/I_Spawner.Deactivate`
  ;[1 1 1] Clears SpawnEnemy timer
  (`KismetSystemLibrary.K2_ClearTimer` null "SpawnEnemy"))

(event `SpawnEnemy`
  (bind (_spawneeclass_type _spawneeclass_scale) (break `/Game/SpaceShooter2DKit/Blueprints/Spawners/STR_EnemySpawnee` (`self.SpawneeClass`)))
  ;[1 1 1] Get all enemies in level
  (bind _outactors (`GameplayStatics.GetAllActorsOfClass` "/Game/SpaceShooter2DKit/Blueprints/Enemies/BP_BaseEnemy.BP_BaseEnemy_C"))
  ;[1 1 1] Filter on spawnee type
  (bind _filteredenemies (`self.FilterOnType` _outactors (`.Type_6_155FAFCB0F403035815DB095C42204E4` (break `/Game/SpaceShooter2DKit/Blueprints/Spawners/STR_EnemySpawnee` (`self.SpawneeClass`)))))
  ;[1 1 1] If true, spawn enemy
  (if (< (`KismetArrayLibrary.Array_Length` _filteredenemies) (`self.MaxSpawneesInLevel`))
    (`self.SpawnEnemyType` _spawneeclass_type _spawneeclass_scale)))

(fn `UserConstructionScript`)