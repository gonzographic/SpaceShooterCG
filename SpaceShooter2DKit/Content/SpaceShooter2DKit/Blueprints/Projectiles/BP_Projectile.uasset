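; BP_Projectile is a configurable 2D shooter projectile that damages what it hits.
; On BeginPlay it applies its collision channel and flipbook to the PaperFlipbook component, then sets the ProjectileMovement velocity in local space from Direction and Speed.
; On a hit with a valid actor it applies Damage, naming itself as the damage causer, and destroys itself.
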(event `self.ReceiveBeginPlay`
  (`PrimitiveComponent.SetCollisionObjectType` (`self.PaperFlipbook`) (`self.CollisionChannel`))
  (`PaperFlipbookComponent.SetFlipbook` (`self.PaperFlipbook`) (`self.Flipbook`))
  (`self.SetVelocity`))

(event `self.ReceiveHit`
  (params (MyComp :type "PrimitiveComponent Object Reference") (Other :type "Actor Object Reference") (OtherComp :type "PrimitiveComponent Object Reference") (bSelfMoved :type Boolean) (HitLocation :type "Vector Structure") (HitNormal :type "Vector Structure") (NormalImpulse :type "Vector Structure") (Hit :type "HitResult Structure (by ref)"))
  (`/Engine/EditorBlueprintResources/StandardMacros.IsValid` Other
    (:`Is Valid`
      (`GameplayStatics.ApplyDamage` Other (`self.Damage`) null self)
      (`self.K2_DestroyActor`))))

(fn `SetVelocity`
  ;[1 1 1] Set velocity (direction * speed)
  (`ProjectileMovementComponent.SetVelocityInLocalSpace` (`self.ProjectileMovement`) (* (`self.Direction`) (`self.Speed`))))

(fn `UserConstructionScript`)