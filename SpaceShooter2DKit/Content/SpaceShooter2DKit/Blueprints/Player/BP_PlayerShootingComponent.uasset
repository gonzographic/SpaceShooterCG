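; Player shooting component for the 2D space shooter that fires projectiles from the owning actor and tracks ammo.
; Tap, Hold and Automatic modes drive FireWeapon directly or through a looping fire-rate timer, with Automatic starting only on TestMap.
; Weapon types come from a Data Table, starting at SingleShot and switchable by index.
; Each shot costs one ammo unless unlimited and spawns a BP_Projectile per eject point, angled from the owner's forward vector.
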(event `self.ReceiveBeginPlay`
  ;[1 1 1] Set weapon types variable and current weapon
  (`self.InitializeWeapons`)
  ;[1 1 1] Initializes the ammo
  (`self.InitializeAmmo`)
  ;[1 1 1] Start automatic firing
  (if (`self.ShouldFireAutomatic`)
    (`self.StartFiring`)))

(event `OnFirePressed`
  ;[1 1 1] Check disabled
  (if (not (`self.Disabled`))
    ;[1 1 1] Fire once for tap, start and release for hold, automatic handled on BeginPlay
    (switch `/Game/SpaceShooter2DKit/Blueprints/Player/ENUM_FireModes` (`self.CurrentFireMode`)
      (:`NewEnumerator0`
        (`self.FireWeapon`))
      (:`NewEnumerator1`
        (`/Engine/EditorBlueprintResources/StandardMacros.DoOnce` false :!label _label
          (:`Completed`
            (`self.FireWeapon`)
            (`self.StartFiring`)))))))

(event `OnFireReleased`
  ;[1 1 1] Fire once for tap, start and release for hold, automatic handled on BeginPlay
  (if (`|EnumEquality` (`self.CurrentFireMode`) "NewEnumerator1")
    (`self.StopFiring`)
    (goto _label :!via `Reset`)))

(fn `ChangeAmmo`
  (params (Delta :type Integer))
  ;[1 1 1] Add delta to current ammo and clamp between 0 and max  ammo
  (set `self.CurrentAmmo` (`KismetMathLibrary.Clamp` (+ (`self.CurrentAmmo`) (`local.Delta`)) 0 (`self.MaxAmmo`))))

(fn `ChangeWeapon`
  (params (Delta :type Integer))
  ;[1 1 1] Add delta and clamp value between 0 and number of weapon type names
  (set `self.WeaponTypeIndex` (`KismetMathLibrary.Clamp` (+ (`self.WeaponTypeIndex`) (`local.Delta`)) 0 (- (`KismetArrayLibrary.Array_Length` (`self.WeaponTypeNames`)) 1)))
  ;[1 1 1] Get the weapon type from the Data Table
  (bind _returnvalue (`|GetDataTableRow` "/Game/SpaceShooter2DKit/Blueprints/Player/DT_PlayerWeaponTypes.DT_PlayerWeaponTypes" (`|GetArrayItem` (`self.WeaponTypeNames`) (`self.WeaponTypeIndex`)))
    (:`then`
      ;[1 1 1] Set the eject mode
      (set `self.CurrentWeaponType` _returnvalue))
    (:`RowNotFound`
      (`KismetSystemLibrary.PrintString` "Invalid WeaponTypeIndex in PlayerShootingComponent" true true (struct :`R` 1.0 :`A` 1.0)))))

(fn `Disable`
  (`self.StopFiring`)
  (set `self.Disabled` true))

(fn `FireWeapon`
  (bind _currentweapontype_ejectpoint (break `/Game/SpaceShooter2DKit/Blueprints/Player/STR_PlayerEjectMode` (`self.CurrentWeaponType`)))
  (if (`self.UnlimitedAmmo`)
    (for _array_element _currentweapontype_ejectpoint :!label _label
      (bind (_verticaloffset _spawnoffset _anglefromforward) (break `/Game/SpaceShooter2DKit/Blueprints/Player/STR_EjectInfo` _array_element))
      (bind _firedirection (`self.GetFireDirection` _anglefromforward))
      ;[1 1 1] Spawn projectiles
      (`|SpawnActorFromClass` "/Game/SpaceShooter2DKit/Blueprints/Projectiles/BP_Projectile.BP_Projectile_C" (`KismetMathLibrary.MakeTransform` (+ (`Actor.K2_GetActorLocation` (`self.GetOwner`)) (+ (* (`Actor.GetActorUpVector` (`self.GetOwner`)) _verticaloffset) (* _firedirection _spawnoffset))) (struct) (`self.ProjectileScale`)) "Undefined" "OverrideRootScale" null _firedirection (`self.ProjectileDamage`) "ECC_GameTraceChannel3" "/Game/SpaceShooter2DKit/Animations/Projectiles/FB_PlayerTorpedo.FB_PlayerTorpedo" null))
    ;[1 1 1] When done, play fire sound
    (`GameplayStatics.PlaySound2D` (`self.FireSound`))
    (else
      ;[1 1 1] Only fire if there is ammo
      (if (`self.HasAmmo`)
        ;[1 1 1] Reduce ammo with 1
        (`self.ChangeAmmo` -1)
        (goto _label)))))

(fn `GetFireDirection`
  (params (AngleFromForward :type "Float (double-precision)"))
  (returns (FireDirection :type "Vector Structure"))
  (return (`KismetMathLibrary.RotateAngleAxis` (`Actor.GetActorForwardVector` (`self.GetOwner`)) (`local.AngleFromForward`) (`Actor.GetActorRightVector` (`self.GetOwner`)))))

(fn `HasAmmo`
  (returns (HasAmmo :type Boolean))
  (return (select `bool` (`self.UnlimitedAmmo`) :`false` (> (`self.CurrentAmmo`) 0) :`true` true)))

(fn `InitializeAmmo`
  ;[1 1 1] Add the start ammo
  (`self.ChangeAmmo` (`self.StartAmmo`)))

(fn `InitializeWeapons`
  ;[1 1 1] Save the Data Table names
  (bind _outrownames (`DataTableFunctionLibrary.GetDataTableRowNames` "/Game/SpaceShooter2DKit/Blueprints/Player/DT_PlayerWeaponTypes.DT_PlayerWeaponTypes"))
  (set `self.WeaponTypeNames` _outrownames)
  ;[1 1 1] Set the current weapon type to SingleShot
  (bind _returnvalue (`|GetDataTableRow` "/Game/SpaceShooter2DKit/Blueprints/Player/DT_PlayerWeaponTypes.DT_PlayerWeaponTypes" "SingleShot")
    (:`then`
      (set `self.CurrentWeaponType` _returnvalue))))

(fn `ShouldFireAutomatic`
  (returns (FireAutomatic :type Boolean))
  ;[1 1 1] Check fire mode
  (if (`|EnumEquality` (`self.CurrentFireMode`) "NewEnumerator2")
    ;[1 1 1] Start firing for Automatic Fire Mode only on TestMap (not Main Menu)
    (bind _returnvalue (`GameplayStatics.GetCurrentLevelName` true))
    (if (== _returnvalue "TestMap")
      (return true)
      (else
        (return false)))
    (else
      (return false))))

(fn `StartFiring`
  ;[1 1 1] Continiously fire weapon with fire rate
  (`KismetSystemLibrary.K2_SetTimer` null "FireWeapon" (/ 1.0 (`self.FireRate`)) true))

(fn `StopFiring`
  ;[1 1 1] Stop firing weapon
  (`KismetSystemLibrary.K2_ClearTimer` null "FireWeapon"))