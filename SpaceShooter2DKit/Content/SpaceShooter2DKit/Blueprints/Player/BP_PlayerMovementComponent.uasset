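; Player movement component for a 2D space shooter that moves its owning actor on the XZ plane.
; ApplyMovementInput normalizes the right and forward inputs into a direction, scales it by MovementSpeed and delta time, and applies a swept world offset to the owner.
; Disable sets a flag that stops further movement; the component shows no way to clear it.
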(fn `ApplyMovementInput`
  (params (DeltaTime :type "Float (double-precision)") (MoveRight :type "Float (double-precision)") (MoveForward :type "Float (double-precision)"))
  ;[1 1 1] Check disabled
  (if (not (`self.Disabled`))
    ;[1 1 1] Apply vector to location
    (`Actor.K2_AddActorWorldOffset` (`self.GetOwner`) (* (`KismetMathLibrary.Normal` (`KismetMathLibrary.MakeVector` (`local.MoveRight`) 0.0 (`local.MoveForward`))) (* (`local.DeltaTime`) (`self.MovementSpeed`))) true false)))

(fn `Disable`
  (set `self.Disabled` true))