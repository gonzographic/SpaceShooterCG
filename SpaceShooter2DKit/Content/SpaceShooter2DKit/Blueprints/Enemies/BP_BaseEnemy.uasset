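; Base enemy actor for the 2D space shooter, configured from the DT_EnemyTypes data table by its type enum.
; On BeginPlay it applies the row's collision box, flipbooks, health and random spin, then initializes movement, shooting and evade components.
; Hitting the player deals collision damage and optionally self-destructs.
; Death disables collision and those components, plays sound and animation, adds score through the game mode, then destroys the actor.
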(event `CustomEvent`)

(event `self.ReceiveBeginPlay`
  ;[1 1 1] Load properties and initialize the enemy
  (`self.LoadProperties`)
  (`self.Initialize`))

(event `self.Box.OnComponentHit`
  (params (HitComponent :type "PrimitiveComponent Object Reference") (OtherActor :type "Actor Object Reference") (OtherComp :type "PrimitiveComponent Object Reference") (NormalImpulse :type "Vector Structure") (Hit :type "HitResult Structure (by ref)"))
  ;[1 1 1] Handle collision with player (deal collision damage player and inflict SelfDestructDamage to self when Dies On Collision is enabled)
  (`/Engine/EditorBlueprintResources/StandardMacros.IsValid` OtherActor
    (:`Is Valid`
      (bind _asbp_player (cast `/Game/SpaceShooter2DKit/Blueprints/Player/BP_Player` OtherActor))
      (`GameplayStatics.ApplyDamage` _asbp_player (`.CollisionDamage_14_6B99E0D9EF4C3F0B70E651A1BC472801` (break `/Game/SpaceShooter2DKit/Blueprints/Enemies/STR_EnemyBasicProperties` (`.BasicProperties_42_E80AA7B9496F165D4D58BF944CCD046E` (break `/Game/SpaceShooter2DKit/Blueprints/Enemies/STR_EnemyProperties` (`self.Properties`))))) (`self.GetController`) self)
      (if (`.DiesOnCollision_37_EA01B6DE48400F3E5BAF628EB103AB5E` (break `/Game/SpaceShooter2DKit/Blueprints/Enemies/STR_EnemyBasicProperties` (`.BasicProperties_42_E80AA7B9496F165D4D58BF944CCD046E` (break `/Game/SpaceShooter2DKit/Blueprints/Enemies/STR_EnemyProperties` (`self.Properties`)))))
        (`GameplayStatics.ApplyDamage` self (`self.SelfDestructDamage`) (`self.GetController`) self)))))

(event `/Game/SpaceShooter2DKit/Blueprints/Components/I_HealthActor.OnDeath`
  (`self.HandleDeath`))

(event `HandleDeath`
  (`|ExecutionSequence`
    (:`then_0`
      ;[1 1 1] Play Death sound
      (`GameplayStatics.PlaySound2D` (`.DeathSound_41_9B78549A4D81F9DC6AF004ABD5932E72` (break `/Game/SpaceShooter2DKit/Blueprints/Enemies/STR_EnemyBasicProperties` (`.BasicProperties_42_E80AA7B9496F165D4D58BF944CCD046E` (break `/Game/SpaceShooter2DKit/Blueprints/Enemies/STR_EnemyProperties` (`self.Properties`)))))))
    (:`then_1`
      ;[1 1 1] Disable collision
      (`PrimitiveComponent.SetCollisionEnabled` (`self.Box`) "NoCollision"))
    (:`then_2`
      ;[1 1 1] Disable components
      (`self.DisableComponents`))
    (:`then_3`
      ;[1 1 1] Hide engine flipbook
      (`SceneComponent.SetVisibility` (`self.EngineFlipbook`) false false))
    (:`then_4`
      ;[1 1 1] Change to Death animation
      (`self.ChangeAnimation` "NewEnumerator1"))
    (:`then_5`
      ;[1 1 1] Update player score
      (`self.UpdateScore`))
    (:`then_6`
      ;[1 1 1] Play Death Animation once, then destroy actor
      (`KismetSystemLibrary.Delay` (`PaperFlipbookComponent.GetFlipbookLength` (`self.ShipFlipbook`)))
      (`self.K2_DestroyActor`))))

(fn `ChangeAnimation`
  (params (AnimationState :type "/Game/SpaceShooter2DKit/Blueprints/Enemies/ENUM_AnimationStates Enum" :default "NewEnumerator0"))
  (bind ((`Animation_53_67AEE9F64344E51E4D6ABB8377D7B0FE` _animation)) (break `/Game/SpaceShooter2DKit/Blueprints/Enemies/STR_EnemyBasicProperties` (`.BasicProperties_42_E80AA7B9496F165D4D58BF944CCD046E` (break `/Game/SpaceShooter2DKit/Blueprints/Enemies/STR_EnemyProperties` (`self.Properties`)))))
  (bind ((`Animation_53_67AEE9F64344E51E4D6ABB8377D7B0FE` _animation_2)) (break `/Game/SpaceShooter2DKit/Blueprints/Enemies/STR_EnemyBasicProperties` (`.BasicProperties_42_E80AA7B9496F165D4D58BF944CCD046E` (break `/Game/SpaceShooter2DKit/Blueprints/Enemies/STR_EnemyProperties` (`self.Properties`)))))
  (bind (_flipbook _transform) (break `/Game/SpaceShooter2DKit/Blueprints/Enemies/STR_Animation` (`.EngineAnimation_14_FEC4B6724958BDE9AA52B2A73DD3BF44` (break `/Game/SpaceShooter2DKit/Blueprints/Enemies/STR_AnimationProperties` (`.Animation_53_67AEE9F64344E51E4D6ABB8377D7B0FE` (break `/Game/SpaceShooter2DKit/Blueprints/Enemies/STR_EnemyBasicProperties` (`.BasicProperties_42_E80AA7B9496F165D4D58BF944CCD046E` (break `/Game/SpaceShooter2DKit/Blueprints/Enemies/STR_EnemyProperties` (`self.Properties`)))))))))
  (`|ExecutionSequence`
    (:`then_0`
      ;[1 1 1] Set correct flipbook
      (`PaperFlipbookComponent.SetFlipbook` (`self.ShipFlipbook`) (select `/Game/SpaceShooter2DKit/Blueprints/Enemies/ENUM_AnimationStates` (`local.AnimationState`) :`NewEnumerator0` (break `/Game/SpaceShooter2DKit/Blueprints/Enemies/STR_Animation` (break `/Game/SpaceShooter2DKit/Blueprints/Enemies/STR_AnimationProperties` _animation)) :`NewEnumerator1` (break `/Game/SpaceShooter2DKit/Blueprints/Enemies/STR_Animation` (`.DeadAnimation_11_CCC32E6F2A427A9BAC2FCF9652C232DB` (break `/Game/SpaceShooter2DKit/Blueprints/Enemies/STR_AnimationProperties` _animation))))))
    (:`then_1`
      ;[1 1 1] Set flipbook transform
      (`SceneComponent.K2_SetRelativeTransform` (`self.ShipFlipbook`) (select `/Game/SpaceShooter2DKit/Blueprints/Enemies/ENUM_AnimationStates` (`local.AnimationState`) :`NewEnumerator0` (`.Transform_11_1B72DF534FE4E8B05BE2CAB01C6C9D90` (break `/Game/SpaceShooter2DKit/Blueprints/Enemies/STR_Animation` (break `/Game/SpaceShooter2DKit/Blueprints/Enemies/STR_AnimationProperties` _animation_2))) :`NewEnumerator1` (`.Transform_11_1B72DF534FE4E8B05BE2CAB01C6C9D90` (break `/Game/SpaceShooter2DKit/Blueprints/Enemies/STR_Animation` (`.DeadAnimation_11_CCC32E6F2A427A9BAC2FCF9652C232DB` (break `/Game/SpaceShooter2DKit/Blueprints/Enemies/STR_AnimationProperties` _animation_2))))) false true))
    (:`then_2`
      ;[1 1 1] Set Engine flipbook and transform
      (`PaperFlipbookComponent.SetFlipbook` (`self.EngineFlipbook`) _flipbook)
      (`SceneComponent.K2_SetRelativeTransform` (`self.EngineFlipbook`) _transform false true))))

(fn `DisableComponents`
  ;[1 1 1] Stop movement
  (`/Game/SpaceShooter2DKit/Blueprints/Enemies/BP_EnemyMovementComponent.Disable` (`self.BP_EnemyMovementComponent`))
  ;[1 1 1] Stop shooting
  (`/Game/SpaceShooter2DKit/Blueprints/Enemies/BP_EnemyShootingComponent.Disable` (`self.BP_EnemyShootingComponent`))
  ;[1 1 1] Stop evading
  (`/Game/SpaceShooter2DKit/Blueprints/Enemies/BP_EnemyEvadeComponent.Disable` (`self.BP_EnemyEvadeComponent`)))

(fn `HasType`
  (params (Type :type "/Game/SpaceShooter2DKit/Blueprints/Enemies/ENUM_EnemyType Enum" :default "NewEnumerator0"))
  (returns (IsType :type Boolean))
  ;[1 1 1] Compare type and return
  (return (`|EnumEquality` Type (`self.Type`))))

(fn `Initialize`
  (`self.InitializeBasicProperties`)
  (`self.InitializeComponents`))

(fn `InitializeBasicProperties`
  (`|ExecutionSequence`
    (:`then_0`
      ;[1 1 1] Set collision size
      (`self.SetBoxCollisionExtent`))
    (:`then_1`
      ;[1 1 1] Set visuals
      (`self.ChangeAnimation` "NewEnumerator0"))
    (:`then_2`
      ;[1 1 1] Setup Health
      (`/Game/SpaceShooter2DKit/Blueprints/Components/BP_HealthComponent.InitializeEnemyHealth` (`self.BP_HealthComponent`) (`.Health_28_ED58F6B64A4A67019C62E0A24D0F75D4` (break `/Game/SpaceShooter2DKit/Blueprints/Enemies/STR_EnemyBasicProperties` (`.BasicProperties_42_E80AA7B9496F165D4D58BF944CCD046E` (break `/Game/SpaceShooter2DKit/Blueprints/Enemies/STR_EnemyProperties` (`self.Properties`)))))))
    (:`then_3`
      ;[1 1 1] Setup rotation
      (`self.SetRotationMovement` (`.Rotation_44_82243ECD493C4BE0B91D5D84BB8843E1` (break `/Game/SpaceShooter2DKit/Blueprints/Enemies/STR_EnemyBasicProperties` (`.BasicProperties_42_E80AA7B9496F165D4D58BF944CCD046E` (break `/Game/SpaceShooter2DKit/Blueprints/Enemies/STR_EnemyProperties` (`self.Properties`)))))))))

(fn `InitializeComponents`
  ;[1 1 1] Initialize movement
  (`/Game/SpaceShooter2DKit/Blueprints/Enemies/BP_EnemyMovementComponent.Initialize` (`self.BP_EnemyMovementComponent`) (`.MovementProperties_34_C7DB77386F492C59FA6EF18FE34C060D` (break `/Game/SpaceShooter2DKit/Blueprints/Enemies/STR_EnemyProperties` (`self.Properties`))))
  ;[1 1 1] Initialize shooting
  (`/Game/SpaceShooter2DKit/Blueprints/Enemies/BP_EnemyShootingComponent.Initialize` (`self.BP_EnemyShootingComponent`) (`.ShootingProperties_45_FB77BBD9D24C5718FFDF45BE31FD1F86` (break `/Game/SpaceShooter2DKit/Blueprints/Enemies/STR_EnemyProperties` (`self.Properties`))))
  ;[1 1 1] Initialize evading
  (`/Game/SpaceShooter2DKit/Blueprints/Enemies/BP_EnemyEvadeComponent.Initialize` (`self.BP_EnemyEvadeComponent`) (`.EvadeProperties_14_A6C086897849DF45B7A90C8586CBCE8E` (break `/Game/SpaceShooter2DKit/Blueprints/Enemies/STR_EnemyProperties` (`self.Properties`)))))

(fn `LoadProperties`
  (bind _returnvalue (`|GetEnumeratorNameAsString` (`self.Type`)))
  ;[1 1 1] Get properties from Data Table using type variable
  (bind _returnvalue_2 (`|GetDataTableRow` "/Game/SpaceShooter2DKit/Blueprints/Enemies/DT_EnemyTypes.DT_EnemyTypes" (`KismetStringLibrary.Conv_StringToName` _returnvalue))
    (:`then`
      ;[1 1 1] If found, set properties
      (set `self.Properties` _returnvalue_2))
    (:`RowNotFound`
      ;[1 1 1] Else, display error message
      (`KismetSystemLibrary.PrintString` (`KismetStringLibrary.Concat_StrStr` _returnvalue "NOT FOUND")))))

(fn `SetBoxCollisionExtent`
  ;[1 1 1] Setup Box extent for collision
  (`BoxComponent.SetBoxExtent` (`self.Box`) (`.CollisionBoxExtent_56_92FD624142465A1678A3FEA76EC79E47` (break `/Game/SpaceShooter2DKit/Blueprints/Enemies/STR_EnemyBasicProperties` (`.BasicProperties_42_E80AA7B9496F165D4D58BF944CCD046E` (break `/Game/SpaceShooter2DKit/Blueprints/Enemies/STR_EnemyProperties` (`self.Properties`))))) true))

(fn `SetRotationMovement`
  (params (RotationRange :type "FloatRange Structure"))
  (bind (_lowerbound _upperbound) (break `FloatRange` RotationRange))
  ;[1 1 1] Pick random float between min and max and set value
  (set `RotatingMovementComponent.RotationRate` (`KismetMathLibrary.MakeRotator` 0.0 (`KismetMathLibrary.RandomFloatInRange` (`.Value` (break `FloatRangeBound` _lowerbound)) (`.Value` (break `FloatRangeBound` _upperbound)))) (`self.RotatingMovement`)))

(fn `ShouldIgnoreDamage`
  (returns (IgnoreDamage :type Boolean))
  ;[1 1 1] Enemy should never ignore damage
  (return false))

(fn `UpdateScore`
  ;[1 1 1] Get 2DSpaceShooter GameMode
  (bind _asbp_space_shooter_2dgame_mode (cast `/Game/SpaceShooter2DKit/Blueprints/Game/BP_SpaceShooter2DGameMode` (`GameplayStatics.GetGameMode`)))
  ;[1 1 1] Change score
  (`/Game/SpaceShooter2DKit/Blueprints/Game/BP_SpaceShooter2DGameMode.ChangeScore` _asbp_space_shooter_2dgame_mode (`.Score_5_789A102BC64469D4362CA69CBB38C344` (break `/Game/SpaceShooter2DKit/Blueprints/Enemies/STR_EnemyBasicProperties` (`.BasicProperties_42_E80AA7B9496F165D4D58BF944CCD046E` (break `/Game/SpaceShooter2DKit/Blueprints/Enemies/STR_EnemyProperties` (`self.Properties`)))))))

(fn `UserConstructionScript`)