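; Movement component for SpaceShooter2DKit enemies that moves its owner with a swept world offset each tick until disabled.
; Initialization stores movement properties and rotates the base direction by a random angle around the owner's right vector.
; Enemies flagged to seek steer toward the player while their X exceeds the player's, otherwise following the base direction.
; A settable direction addition biases the result, and speed is not scaled by delta time.
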(event `self.ReceiveTick`
  (params (DeltaSeconds :type "Float (single-precision)"))
  ;[1 1 1] Move when not disabled
  (if (not (`self.Disabled`))
    (`Actor.K2_AddActorWorldOffset` (`self.GetOwner`) (* (`self.GetMoveDirection`) (`.MovementSpeed_37_2E7E10D8470E6196C7453ABEE6D8F6FB` (break `/Game/SpaceShooter2DKit/Blueprints/Enemies/STR_EnemyMovementProperties` (`self.MovementProperties`)))) true false)))

(fn `ClearDirectionAddition`
  ;[1 1 1] Reset the direction multiplier to the default value
  (set `self.DirectionAddition` (defaults `/Game/SpaceShooter2DKit/Blueprints/Enemies/BP_EnemyMovementComponent` "BP_EnemyMovementComponent_C")))

(fn `Disable`
  (set `self.Disabled` true))

(fn `GetMoveDirection`
  (returns (MoveDirection :type "Vector Structure"))
  (return (`KismetMathLibrary.Normal` (+ (select `bool` (`self.ShouldMoveToPlayer`) :`false` (`self.BaseMovementDirection`) :`true` (`self.GetPlayerDirection`)) (`self.DirectionAddition`)))))

(fn `GetPlayerDirection`
  (returns (ToPlayerDirection :type "Vector Structure"))
  (return (`KismetMathLibrary.Normal` (- (`Actor.K2_GetActorLocation` (`GameplayStatics.GetPlayerPawn` 0)) (`Actor.K2_GetActorLocation` (`self.GetOwner`))))))

(fn `Initialize`
  (params (MovementProperties :type "/Game/SpaceShooter2DKit/Blueprints/Enemies/STR_EnemyMovementProperties Structure"))
  (set `self.MovementProperties` MovementProperties)
  (`self.InitializeBaseMovementDirection`))

(fn `InitializeBaseMovementDirection`
  (bind (_lowerbound _upperbound) (break `FloatRange` (`.MovementAngle_36_D3BFF23A47D305A50D67CB9032856EAD` (break `/Game/SpaceShooter2DKit/Blueprints/Enemies/STR_EnemyMovementProperties` (`self.MovementProperties`)))))
  (set `self.BaseMovementDirection` (`KismetMathLibrary.Normal` (`KismetMathLibrary.RotateAngleAxis` (`self.BaseMovementDirection`) (`KismetMathLibrary.RandomFloatInRange` (`.Value` (break `FloatRangeBound` _lowerbound)) (`.Value` (break `FloatRangeBound` _upperbound))) (`Actor.GetActorRightVector` (`self.GetOwner`))))))

(fn `IsInFrontOfPlayer`
  (returns (IsInFront :type Boolean))
  (return (> (.x (`Actor.K2_GetActorLocation` (`self.GetOwner`))) (.x (`Actor.K2_GetActorLocation` (`GameplayStatics.GetPlayerPawn` 0))))))

(fn `SetDirectionAddition`
  (params (DirectionMultiplier :type "Vector Structure"))
  (set `self.DirectionAddition` DirectionMultiplier))

(fn `ShouldMoveToPlayer`
  (returns (MoveToPlayer :type Boolean))
  (return (and (`.MoveToPlayer_32_9B2580764185EAF2DEB702A14DE2B163` (break `/Game/SpaceShooter2DKit/Blueprints/Enemies/STR_EnemyMovementProperties` (`self.MovementProperties`))) (`self.IsInFrontOfPlayer`))))